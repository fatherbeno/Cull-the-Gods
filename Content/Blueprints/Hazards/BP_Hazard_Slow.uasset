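; BP_Hazard_Slow is a hazard volume that slows a ThirdPersonCharacter while it overlaps the Box component.
; Begin overlap casts the other actor and sets its CharacterMovement MaxWalkSpeed to a fixed reduced value.
; End overlap adds a fixed amount to the current MaxWalkSpeed instead of restoring a saved original.
; Both events print debug strings for the speed change or a failed cast.
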(event OnComponentBeginOverlap(Box)
  (params (OverlappedComponent :type Primitive%20Component%20Object%20Reference) (OtherActor :type Actor%20Object%20Reference) (OtherComp :type Primitive%20Component%20Object%20Reference) (OtherBodyIndex :type Integer) (bFromSweep :type Boolean) (SweepResult :type Hit%20Result%20Structure%20%28by%20ref%29))
  (bind _asthird_person_character (Utilities|Casting|CastToThirdPersonCharacter OtherActor)
    (:then
      (Variables|/Script/Engine.CharacterMovementComponent|SetMaxWalkSpeed (Variables|/Script/Engine.Character|GetCharacterMovement _asthird_person_character) 3e+02)
      (Development|PrintString "movement speed reduced"))
    (:CastFailed
      (Development|PrintString "Cast Failed"))))

(event OnComponentEndOverlap(Box)
  (params (OverlappedComponent :type Primitive%20Component%20Object%20Reference) (OtherActor :type Actor%20Object%20Reference) (OtherComp :type Primitive%20Component%20Object%20Reference) (OtherBodyIndex :type Integer))
  (bind _asthird_person_character (Utilities|Casting|CastToThirdPersonCharacter OtherActor)
    (:then
      (Variables|/Script/Engine.CharacterMovementComponent|SetMaxWalkSpeed (Variables|/Script/Engine.Character|GetCharacterMovement _asthird_person_character) (+ 3e+02 (Variables|/Script/Engine.CharacterMovementComponent|GetMaxWalkSpeed (Variables|/Script/Engine.Character|GetCharacterMovement _asthird_person_character))))
      (Development|PrintString "movement speed is normal"))
    (:CastFailed
      (Development|PrintString "Cast end Failed"))))

(fn ConstructionScript)