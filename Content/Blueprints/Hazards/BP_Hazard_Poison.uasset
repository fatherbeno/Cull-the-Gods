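; Poison hazard volume that deals damage over time to the third-person player character while it stands inside.
; Box overlap begin sets an in-radius flag and runs a delay-driven loop that subtracts Health on each tick until the player leaves or Health runs out.
; Overlap end clears the flag to stop the loop.
; Death and damage only print debug messages.
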(event OnComponentBeginOverlap(Box)
  (params (OverlappedComponent :type Primitive%20Component%20Object%20Reference) (OtherActor :type Actor%20Object%20Reference) (OtherComp :type Primitive%20Component%20Object%20Reference) (OtherBodyIndex :type Integer) (bFromSweep :type Boolean) (SweepResult :type Hit%20Result%20Structure%20%28by%20ref%29))
  (bind _asthird_person_character (Utilities|Casting|CastToThirdPersonCharacter OtherActor)
    (:then
      (Variables|Default|SetPlayerInRadius true)
      (bind _output_get (Variables|/Game/ThirdPersonBP/Blueprints/ThirdPersonCharacter.ThirdPersonCharacter_C|SetHealth _asthird_person_character (- (Variables|/Game/ThirdPersonBP/Blueprints/ThirdPersonCharacter.ThirdPersonCharacter_C|GetHealth _asthird_person_character) 1.0) :!label _label))
      (Development|PrintString "Damage taken")
      (if (<= _output_get 0.0)
        (Development|PrintString "Death.")
        (else
          (Utilities|FlowControl|Delay 0.5)
          (if (Variables|Default|GetPlayerInRadius)
            (goto _label)))))
    (:CastFailed
      (Development|PrintString "Cast Failed, DoT"))))

(event OnComponentEndOverlap(Box)
  (params (OverlappedComponent :type Primitive%20Component%20Object%20Reference) (OtherActor :type Actor%20Object%20Reference) (OtherComp :type Primitive%20Component%20Object%20Reference) (OtherBodyIndex :type Integer))
  (Utilities|Casting|CastToThirdPersonCharacter OtherActor)
  (Variables|Default|SetPlayerInRadius false))

(fn ConstructionScript)