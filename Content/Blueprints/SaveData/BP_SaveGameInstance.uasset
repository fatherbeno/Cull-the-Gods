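; Game instance that loads or creates the player save data at startup and applies sound options.
; Init loads the save slot, or creates BP_PlayerSaveData and fires the options setup dispatcher.
; After fixed delays, if the current level is Lvl_Loading, it dispatches saved options and opens Lvl_MainMenu.
; A bound listener maps slider volumes into sound-class overrides on the CTG_SCM mix.
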(event Custom|ApplySoundOptions
  (params (MasterVolume :type Float%20%28single-precision%29) (MusicVolume :type Float%20%28single-precision%29) (SFX%20Volume :type Float%20%28single-precision%29) (VoicesVolume :type Float%20%28single-precision%29) (AmbientVolume :type Float%20%28single-precision%29) (MenuVolume :type Float%20%28single-precision%29))
  (Audio|SetSoundMixClassOverride "/Game/Audio/CTG_SCM.CTG_SCM" "/Game/Audio/CTG_SoundClass_Master.CTG_SoundClass_Master" (Math|Float|MapRangeClamped MasterVolume 1e+02 0.0 1.0 0.0) 1.0 0.0 true)
  (Audio|SetSoundMixClassOverride "/Game/Audio/CTG_SCM.CTG_SCM" "/Game/Audio/CTG_SoundClass_Music.CTG_SoundClass_Music" (Math|Float|MapRangeClamped MusicVolume 1e+02 0.0 1.0 0.0) 1.0 0.0 true)
  (Audio|SetSoundMixClassOverride "/Game/Audio/CTG_SCM.CTG_SCM" "/Game/Audio/CTG_SoundClass_SFX.CTG_SoundClass_SFX" (Math|Float|MapRangeClamped SFX%20Volume 1e+02 0.0 1.0 0.0) 1.0 0.0 true)
  (Audio|SetSoundMixClassOverride "/Game/Audio/CTG_SCM.CTG_SCM" "/Game/Audio/CTG_SoundClass_Voices.CTG_SoundClass_Voices" (Math|Float|MapRangeClamped VoicesVolume 1e+02 0.0 1.0 0.0) 1.0 0.0 true)
  (Audio|SetSoundMixClassOverride "/Game/Audio/CTG_SCM.CTG_SCM" "/Game/Audio/CTG_SoundClass_Ambient.CTG_SoundClass_Ambient" (Math|Float|MapRangeClamped AmbientVolume 1e+02 0.0 1.0 0.0) 1.0 0.0 true)
  (Audio|SetSoundMixClassOverride "/Game/Audio/CTG_SCM.CTG_SCM" "/Game/Audio/CTG_SoundClass_Menu.CTG_SoundClass_Menu" (Math|Float|MapRangeClamped MenuVolume 1e+02 0.0 1.0 0.0) 1.0 0.0 true))

(event EventInit
  (EventDispatchers|BindEventtoEventListenerApplySoundOptions (delegate Custom|ApplySoundOptions))
  (bind _returnvalue (SaveGame|DoesSaveGameExist (Variables|Default|GetSaveGameSlot)))
  (if _returnvalue
    (CallFunction|LoadGame)
    (Utilities|FlowControl|Delay 1.0)
    (else
      (bind _returnvalue_2 (SaveGame|CreateSaveGameObject "/Game/Blueprints/SaveData/BP_PlayerSaveData.BP_PlayerSaveData_C"))
      (Variables|Default|SetSaveGameData _returnvalue_2)
      (Utilities|FlowControl|Delay 1.0)
      (Default|CallEventDispatcherSetupOptionsData)))
  (Utilities|FlowControl|Delay 1.0)
  (bind _returnvalue_3 (Game|GetCurrentLevelName true))
  (if (Utilities|Enum|Equal(Enum) _returnvalue_3 "Lvl_Loading")
    (Default|CallEventDispatcherApplySavedOptions)
    (Utilities|FlowControl|Delay 1.0)
    (Game|OpenLevel(byName) "Lvl_MainMenu")))

(fn LoadGame
  (bind _returnvalue (SaveGame|LoadGamefromSlot (Variables|Default|GetSaveGameSlot)))
  (bind _asbp_player_save_data (Utilities|Casting|CastToBP_PlayerSaveData _returnvalue))
  (Variables|Default|SetSaveGameData _asbp_player_save_data)
  (return))