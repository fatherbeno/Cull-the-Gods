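; Spinning boss attack actor that damages anything except Level1Boss_BP overlapping its capsules or ring.
; On BeginPlay it plays audio and an ActorSequence in reverse, waiting briefly before enabling overlap on the capsules and blocking on the ring.
; A delay loop gradually ramps RotatingMovement yaw speed to a cap.
; After a timed hold it plays the sequence forward, disables collision, stops audio and destroys itself.
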(event OnComponentBeginOverlap(Capsule)
  (params (OverlappedComponent :type Primitive%20Component%20Object%20Reference) (OtherActor :type Actor%20Object%20Reference) (OtherComp :type Primitive%20Component%20Object%20Reference) (OtherBodyIndex :type Integer) (bFromSweep :type Boolean) (SweepResult :type Hit%20Result%20Structure%20%28by%20ref%29))
  (bind _returnvalue (Actor|GetActorOfClass "/Game/Blueprints/Boss/Level1Boss_BP.Level1Boss_BP_C"))
  (if (!= OtherActor _returnvalue)
    (Game|Damage|ApplyDamage OtherActor 15.0 0 0)))

(event OnComponentBeginOverlap(Capsule1)
  (params (OverlappedComponent :type Primitive%20Component%20Object%20Reference) (OtherActor :type Actor%20Object%20Reference) (OtherComp :type Primitive%20Component%20Object%20Reference) (OtherBodyIndex :type Integer) (bFromSweep :type Boolean) (SweepResult :type Hit%20Result%20Structure%20%28by%20ref%29))
  (bind _returnvalue (Actor|GetActorOfClass "/Game/Blueprints/Boss/Level1Boss_BP.Level1Boss_BP_C"))
  (if (!= OtherActor _returnvalue)
    (Game|Damage|ApplyDamage OtherActor 15.0 0 0)))

(event OnComponentBeginOverlap(Capsule2)
  (params (OverlappedComponent :type Primitive%20Component%20Object%20Reference) (OtherActor :type Actor%20Object%20Reference) (OtherComp :type Primitive%20Component%20Object%20Reference) (OtherBodyIndex :type Integer) (bFromSweep :type Boolean) (SweepResult :type Hit%20Result%20Structure%20%28by%20ref%29))
  (bind _returnvalue (Actor|GetActorOfClass "/Game/Blueprints/Boss/Level1Boss_BP.Level1Boss_BP_C"))
  (if (!= 0 _returnvalue)
    (Game|Damage|ApplyDamage OtherActor 15.0 0 0)))

(event OnComponentBeginOverlap(Capsule3)
  (params (OverlappedComponent :type Primitive%20Component%20Object%20Reference) (OtherActor :type Actor%20Object%20Reference) (OtherComp :type Primitive%20Component%20Object%20Reference) (OtherBodyIndex :type Integer) (bFromSweep :type Boolean) (SweepResult :type Hit%20Result%20Structure%20%28by%20ref%29))
  (bind _returnvalue (Actor|GetActorOfClass "/Game/Blueprints/Boss/Level1Boss_BP.Level1Boss_BP_C"))
  (if (!= OtherActor _returnvalue)
    (Game|Damage|ApplyDamage OtherActor 15.0 0 0)))

(event OnComponentBeginOverlap(Sphere)
  (params (OverlappedComponent :type Primitive%20Component%20Object%20Reference) (OtherActor :type Actor%20Object%20Reference) (OtherComp :type Primitive%20Component%20Object%20Reference) (OtherBodyIndex :type Integer) (bFromSweep :type Boolean) (SweepResult :type Hit%20Result%20Structure%20%28by%20ref%29)))

(event OnComponentBeginOverlap(Ring)
  (params (OverlappedComponent :type Primitive%20Component%20Object%20Reference) (OtherActor :type Actor%20Object%20Reference) (OtherComp :type Primitive%20Component%20Object%20Reference) (OtherBodyIndex :type Integer) (bFromSweep :type Boolean) (SweepResult :type Hit%20Result%20Structure%20%28by%20ref%29))
  (bind _returnvalue (Actor|GetActorOfClass "/Game/Blueprints/Boss/Level1Boss_BP.Level1Boss_BP_C"))
  (if (!= OtherActor _returnvalue)
    (Game|Damage|ApplyDamage OtherActor 15.0 0 0)))

(event EventBeginPlay
  (bind _rotatingmovement (Variables|Default|GetRotatingMovement))
  (bind _capsule (Variables|Default|GetCapsule))
  (bind _capsule1 (Variables|Default|GetCapsule1))
  (bind _capsule2 (Variables|Default|GetCapsule2))
  (bind _capsule3 (Variables|Default|GetCapsule3))
  (bind _array (Utilities|Array|MakeArray _capsule1 _capsule2 _capsule3 _capsule))
  (Audio|Components|Audio|Play (Variables|Default|GetAudio) 0.0)
  (Class|MovieSceneSequencePlayer|PlayReverse (Variables|/Script/ActorSequence.ActorSequenceComponent|GetSequencePlayer (Variables|Default|GetActorSequence)))
  (Utilities|FlowControl|Delay 2.5)
  ;[1 1 1] Sets collision profiles after few secs to give player chance to get in position
  (Variables|Default|SetCapsule%20Array _array)
  (for _array_element _array
    (Collision|SetCollisionProfileName _array_element "OverlapAllDynamic" true :!class /Script/Engine.PrimitiveComponent)
    (Collision|SetCollisionProfileName (Variables|Default|GetRing) "BlockAll" true :!class /Script/Engine.PrimitiveComponent)
    ;[1 1 1] Adds movement slowly till rate is 20 Z
    (if (<= (.yaw (Variables|/Script/Engine.RotatingMovementComponent|GetRotationRate _rotatingmovement)) 4e+01) :!label _label
      (Variables|/Script/Engine.RotatingMovementComponent|SetRotationRate _rotatingmovement (Math|Rotator|MakeRotator 0.0 0.0 (+ (.yaw (Variables|/Script/Engine.RotatingMovementComponent|GetRotationRate _rotatingmovement)) 2.0)))
      (Utilities|FlowControl|Delay 0.3)
      (goto _label)
      (else
        (Utilities|FlowControl|Delay 1e+01)
        (Collision|SetCollisionProfileName (Variables|Default|GetRing) "NoCollision" true :!class /Script/Engine.PrimitiveComponent)
        (Sequencer|Player|Play (Variables|/Script/ActorSequence.ActorSequenceComponent|GetSequencePlayer (Variables|Default|GetActorSequence)) :!class /Script/MovieScene.MovieSceneSequencePlayer)
        (for _array_element_2 (Variables|Default|GetCapsule%20Array)
          (Collision|SetCollisionProfileName _array_element_2 "NoCollision" true :!class /Script/Engine.PrimitiveComponent)
          (Utilities|FlowControl|Delay 2.0)
          (Audio|Components|Audio|Stop (Variables|Default|GetAudio))
          (Actor|DestroyActor))))))

(fn ConstructionScript)