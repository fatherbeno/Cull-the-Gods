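; BP_FinalGroundOrbs is a boss-attack actor that spawns a set of ground orbs intended to have distinct colours.
; On BeginPlay it spawns a BP_GroundOrb at each of four scene component transforms and adds its colour name to an array with AddUnique.
; A duplicate result destroys that orb and loops back to spawn another at the same spot, with each result printed as long-lasting debug text.
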(event EventBeginPlay
  (bind _colourarray (Variables|Default|GetColourArray))
  (bind _output_get (Variables|Default|SetMy%20Array (Utilities|Array|MakeArray (Variables|Default|GetScene) (Variables|Default|GetScene1) (Variables|Default|GetScene2) (Variables|Default|GetScene3))))
  (for _array_element _output_get
    (bind _returnvalue (Game|SpawnActorfromClass "/Game/Blueprints/Boss/Boss_Attacks/BP_GroundOrb.BP_GroundOrb_C" (Transformation|GetWorldTransform _array_element) "Undefined" 0 0 :!label _label))
    (bind _returnvalue_2 (Utilities|Array|AddUnique _colourarray (Variables|/Game/Blueprints/Boss/Boss_Attacks/BP_GroundOrb.BP_GroundOrb_C|Getcolourname _returnvalue)))
    (Development|PrintString (Utilities|String|ToString(Integer) _returnvalue_2) true true "(R=0.000000,G=0.660000,B=1.000000,A=1.000000)" 222222221312.0)
    (if (== _returnvalue_2 -1)
      (Utilities|Array|RemoveItem _colourarray (Utilities|Array|Get(acopy) _colourarray -1))
      (Actor|DestroyActor _returnvalue)
      (goto _label))))

(fn ConstructionScript)