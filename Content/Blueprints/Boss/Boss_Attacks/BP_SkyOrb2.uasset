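; BP_SkyOrb2 is a boss attack projectile that homes in on the player and destroys itself after a fixed lifetime.
; BeginPlay caches the ThirdPersonCharacter and sets the player pawn's root as the ProjectileMovement homing target.
; Sphere overlaps damage any actor except the owner, unless the player's IsInOrb flag is set, which only prints a debug message.
; The orb is not destroyed on overlap.
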(event OnComponentBeginOverlap(Sphere1)
  (params (OverlappedComponent :type Primitive%20Component%20Object%20Reference) (OtherActor :type Actor%20Object%20Reference) (OtherComp :type Primitive%20Component%20Object%20Reference) (OtherBodyIndex :type Integer) (bFromSweep :type Boolean) (SweepResult :type Hit%20Result%20Structure%20%28by%20ref%29))
  (bind _returnvalue (Components|GetOwner))
  (if (not (== OtherActor _returnvalue))
    ;[1 1 1] ifin circle
    (if (Variables|/Game/ThirdPersonBP/Blueprints/ThirdPersonCharacter.ThirdPersonCharacter_C|GetisInOrb (Variables|Default|GetPlayer%20Reference))
      (Development|PrintString "Player was in circle, no bug" true true "(R=1.000000,G=0.000000,B=0.008232,A=1.000000)")
      (else
        (Game|Damage|ApplyDamage OtherActor 1e+01 0 _returnvalue)))))

(event EventBeginPlay
  ;[1 1 1] set colour and colourname
  (|CallParentFunction)
  (bind _returnvalue (Actor|GetActorOfClass "/Game/ThirdPersonBP/Blueprints/ThirdPersonCharacter.ThirdPersonCharacter_C"))
  (Variables|Default|SetPlayer%20Reference _returnvalue)
  (Variables|/Script/Engine.ProjectileMovementComponent|SetHomingTargetComponent (Variables|Default|GetProjectileMovement) (Variables|/Script/Engine.Actor|GetRootComponent (Game|Player|GetPlayerPawn 0)))
  (Utilities|FlowControl|Delay 7.0)
  (Actor|DestroyActor))

(event EventTick
  (params (DeltaSeconds :type Float%20%28single-precision%29)))

(fn ConstructionScript
  (|CallParentFunction))