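; BP_SandClaw is a short-lived boss attack hitbox with a particle effect that deals fixed damage to overlapping actors other than its owner.
; On BeginPlay it enables capsule overlaps and finds the boss by class, then disables collision and destroys itself after a brief delay.
; Each Tick snaps the particle system to the boss's right-hand socket with an offset roll; the BeginPlay attach call names no parent.
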(event OnComponentBeginOverlap(Capsule)
  (params (OverlappedComponent :type Primitive%20Component%20Object%20Reference) (OtherActor :type Actor%20Object%20Reference) (OtherComp :type Primitive%20Component%20Object%20Reference) (OtherBodyIndex :type Integer) (bFromSweep :type Boolean) (SweepResult :type Hit%20Result%20Structure%20%28by%20ref%29))
  (bind _returnvalue (Components|GetOwner))
  (if (not (== OtherActor _returnvalue))
    (Game|Damage|ApplyDamage OtherActor 1e+01 0 _returnvalue)))

(event EventBeginPlay
  (Collision|SetCollisionProfileName (Variables|Default|GetCapsule) "OverlapAllDynamic" true :!class /Script/Engine.PrimitiveComponent)
  (bind _returnvalue (Actor|GetActorOfClass "/Game/Blueprints/Boss/Boss_Class.Boss_Class_C"))
  (Transformation|AttachComponentToComponent (Variables|/Script/Engine.Actor|GetRootComponent _returnvalue) 0 "hand_rSocket" "KeepWorld" "KeepWorld" "KeepWorld" true)
  (Utilities|FlowControl|Delay 1.3)
  (Collision|SetCollisionProfileName (Variables|Default|GetCapsule) "NoCollision" true :!class /Script/Engine.PrimitiveComponent)
  (Actor|DestroyActor))

(event EventTick
  (params (DeltaSeconds :type Float%20%28single-precision%29))
  (Transformation|SetWorldLocationAndRotation (Variables|Default|GetParticleSystem) (Math|Vector|MakeVector (.x (Transformation|GetSocketLocation (Variables|/Script/Engine.Character|GetMesh (stale EventBeginPlay _returnvalue)) (Class|SkinnedMeshComponent|GetSocketBoneName (Variables|/Script/Engine.Character|GetMesh (stale EventBeginPlay _returnvalue)) "hand_rSocket"))) (.y (Transformation|GetSocketLocation (Variables|/Script/Engine.Character|GetMesh (stale EventBeginPlay _returnvalue)) (Class|SkinnedMeshComponent|GetSocketBoneName (Variables|/Script/Engine.Character|GetMesh (stale EventBeginPlay _returnvalue)) "hand_rSocket"))) (.z (Transformation|GetSocketLocation (Variables|/Script/Engine.Character|GetMesh (stale EventBeginPlay _returnvalue)) (Class|SkinnedMeshComponent|GetSocketBoneName (Variables|/Script/Engine.Character|GetMesh (stale EventBeginPlay _returnvalue)) "hand_rSocket")))) (Math|Rotator|MakeRotator (- (.roll (Transformation|GetSocketRotation (Variables|/Script/Engine.Character|GetMesh (stale EventBeginPlay _returnvalue)) (Class|SkinnedMeshComponent|GetSocketBoneName (Variables|/Script/Engine.Character|GetMesh (stale EventBeginPlay _returnvalue)) "hand_rSocket"))) 1.8e+02) (.pitch (Transformation|GetSocketRotation (Variables|/Script/Engine.Character|GetMesh (stale EventBeginPlay _returnvalue)) (Class|SkinnedMeshComponent|GetSocketBoneName (Variables|/Script/Engine.Character|GetMesh (stale EventBeginPlay _returnvalue)) "hand_rSocket"))) (.yaw (Transformation|GetSocketRotation (Variables|/Script/Engine.Character|GetMesh (stale EventBeginPlay _returnvalue)) (Class|SkinnedMeshComponent|GetSocketBoneName (Variables|/Script/Engine.Character|GetMesh (stale EventBeginPlay _returnvalue)) "hand_rSocket")))) false false))

(fn ConstructionScript)