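; BP_GroundOrb is a ground orb actor, filed under boss attacks, that takes one of four random colours: red, blue, yellow or green.
; On BeginPlay it stores the colour and its name and pushes the colour to the Fx component's "color" parameter.
; Capsule overlaps with any actor except its owner only print the colour name, with no damage or other effect.
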(event OnComponentBeginOverlap(Capsule)
  (params (OverlappedComponent :type Primitive%20Component%20Object%20Reference) (OtherActor :type Actor%20Object%20Reference) (OtherComp :type Primitive%20Component%20Object%20Reference) (OtherBodyIndex :type Integer) (bFromSweep :type Boolean) (SweepResult :type Hit%20Result%20Structure%20%28by%20ref%29))
  (if (not (== OtherActor (Components|GetOwner)))
    (Development|PrintString (Utilities|String|ToString(Name) (Variables|Default|Getcolourname)))))

(event EventBeginPlay
  (|CallParentFunction)
  (switch int (Math|Random|RandomIntegerinRange 0 3)
    (:0
      (Development|PrintString "red")
      (Variables|Default|Setcolour "(R=1.000000,G=0.015783,B=0.000000,A=1.000000)")
      (Effects|Components|ParticleSystem|SetVectorParameter (Variables|Default|Getfx) "color" (Math|Conversions|ToVector(LinearColor) (Variables|Default|Getcolour)))
      (Variables|Default|Setcolourname "red"))
    (:1
      (Development|PrintString "blue")
      (Variables|Default|Setcolour "(R=0.014323,G=0.000000,B=1.000000,A=1.000000)")
      (Effects|Components|ParticleSystem|SetVectorParameter (Variables|Default|Getfx) "color" (Math|Conversions|ToVector(LinearColor) (Variables|Default|Getcolour)))
      (Variables|Default|Setcolourname "blue"))
    (:2
      (Development|PrintString "yellow")
      (Variables|Default|Setcolour "(R=1.000000,G=0.689642,B=0.000000,A=1.000000)")
      (Effects|Components|ParticleSystem|SetVectorParameter (Variables|Default|Getfx) "color" (Math|Conversions|ToVector(LinearColor) (Variables|Default|Getcolour)))
      (Variables|Default|Setcolourname "yellow"))
    (:3
      (Development|PrintString "green")
      (Variables|Default|Setcolour "(R=0.000000,G=1.000000,B=0.083799,A=1.000000)")
      (Effects|Components|ParticleSystem|SetVectorParameter (Variables|Default|Getfx) "color" (Math|Conversions|ToVector(LinearColor) (Variables|Default|Getcolour)))
      (Variables|Default|Setcolourname "green"))))

(event Collision|EventActorBeginOverlap
  (params (OtherActor :type Actor%20Object%20Reference))
  (|CallParentFunction OtherActor) ; This node is disabled and will not be called.\nDrag off pins to build functionality.
)

(event EventTick
  (params (DeltaSeconds :type Float%20%28single-precision%29))
  (|CallParentFunction DeltaSeconds) ; This node is disabled and will not be called.\nDrag off pins to build functionality.
)

(fn ConstructionScript)