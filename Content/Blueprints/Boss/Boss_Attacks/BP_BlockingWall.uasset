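; Wall actor for the Level 1 boss fight that appears and retracts in response to the boss's StartShieldAttack event.
; Each event alternates between showing the cube with a charge sound and forward ActorSequence, and reversing the sequence before hiding it.
; Delays stagger the box's switch between overlap and no collision.
; A looping damage-over-time branch for the player is present but never runs.
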(event Custom|SpawnWalls
  (Utilities|FlowControl|FlipFlop
    (:A
      (Development|SetHiddeninGame (Variables|Default|GetCube) false false)
      (Audio|PlaySoundatLocation "/Game/Audio/SFX/SoundCues/SC_SFX_Boss_SpecialAttackCharge_Long.SC_SFX_Boss_SpecialAttackCharge_Long" (Transformation|GetWorldLocation (Variables|Default|GetCube)) "0, 0, 0" 1.0 1.0 0.0 0 0 0)
      (Sequencer|Player|Play (Variables|/Script/ActorSequence.ActorSequenceComponent|GetSequencePlayer (Variables|Default|GetActorSequence)) :!class /Script/MovieScene.MovieSceneSequencePlayer)
      (Utilities|FlowControl|Delay 3.0)
      (Collision|SetCollisionProfileName (Variables|Default|GetBox) "OverlapAllDynamic" true :!class /Script/Engine.PrimitiveComponent))
    (:B
      (Class|MovieSceneSequencePlayer|PlayReverse (Variables|/Script/ActorSequence.ActorSequenceComponent|GetSequencePlayer (Variables|Default|GetActorSequence)))
      (Utilities|FlowControl|Delay 2.0)
      (Development|SetHiddeninGame (Variables|Default|GetCube) true true)
      (Utilities|FlowControl|Delay 2.0)
      (Collision|SetCollisionProfileName (Variables|Default|GetBox) "NoCollision" true :!class /Script/Engine.PrimitiveComponent))))

(event EventBeginPlay
  (bind _returnvalue (Actor|GetActorOfClass "/Game/Blueprints/Boss/Level1Boss_BP.Level1Boss_BP_C"))
  (EventDispatchers|BindEventtoStartShieldAttack _returnvalue (delegate Custom|SpawnWalls)))

(fn ConstructionScript)