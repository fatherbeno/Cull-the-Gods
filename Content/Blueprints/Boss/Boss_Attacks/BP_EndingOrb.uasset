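; BP_EndingOrb is a boss-attack orb actor with a fixed yellow look, driven by an Actor Sequence.
; On BeginPlay it overrides its colour and colour name to yellow, pushes the colour into the Fx "color" vector parameter, then plays the sequence.
; The delayed self-destroy and the construction-script colour setup, including its parent call, are disconnected and never run.
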(event EventBeginPlay
  (Variables|Default|Setcolour "(R=1.000000,G=0.689642,B=0.000000,A=1.000000)")
  (Effects|Components|ParticleSystem|SetVectorParameter (Variables|Default|Getfx) "color" (Math|Conversions|ToVector(LinearColor) (Variables|Default|Getcolour)))
  (Variables|Default|Setcolourname "yellow")
  (Sequencer|Player|Play (Variables|/Script/ActorSequence.ActorSequenceComponent|GetSequencePlayer (Variables|Default|GetActorSequence)) :!class /Script/MovieScene.MovieSceneSequencePlayer))

(fn ConstructionScript)