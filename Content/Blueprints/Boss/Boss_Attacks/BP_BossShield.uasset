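; BP_BossShield is a boss attack shield with a box hitbox that damages actors overlapping it.
; ChangeCollision flip-flops the box between overlap-all and no collision.
; On overlap it applies fixed damage credited to its owner, skipping that owner and the first Boss_Class actor found.
; The binding of ChangeCollision to Level1Boss_BP's shield attack event is disconnected, and BeginPlay is empty.
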(event OnComponentBeginOverlap(Box)
  (params (OverlappedComponent :type Primitive%20Component%20Object%20Reference) (OtherActor :type Actor%20Object%20Reference) (OtherComp :type Primitive%20Component%20Object%20Reference) (OtherBodyIndex :type Integer) (bFromSweep :type Boolean) (SweepResult :type Hit%20Result%20Structure%20%28by%20ref%29))
  (bind _returnvalue (Components|GetOwner))
  (if (not (== OtherActor _returnvalue))
    (bind _returnvalue_2 (Actor|GetActorOfClass "/Game/Blueprints/Boss/Boss_Class.Boss_Class_C"))
    (if (!= _returnvalue_2 OtherActor)
      (Game|Damage|ApplyDamage OtherActor 15.0 0 _returnvalue))))

(event Custom|ChangeCollision
  (Utilities|FlowControl|FlipFlop
    (:A
      (Collision|SetCollisionProfileName (Variables|Default|GetBox) "OverlapAllDynamic" true :!class /Script/Engine.PrimitiveComponent))
    (:B
      (Collision|SetCollisionProfileName (Variables|Default|GetBox) "NoCollision" true :!class /Script/Engine.PrimitiveComponent))))

(event EventBeginPlay)

(fn ConstructionScript)