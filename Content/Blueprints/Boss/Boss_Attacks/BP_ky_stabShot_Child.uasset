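; BP_ky_stabShot_Child is a homing boss projectile, a coloured sky orb that the player negates by being in the matching colour.
; On spawn it picks red, blue, yellow or green at random, tints its FX, homes on the player pawn and self-destroys after a timed delay.
; Overlapping any actor except its owner deals damage, unless the orb's colour name equals the player's ColourPlayerIsIn.
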(event OnComponentBeginOverlap(Sphere1)
  (params (OverlappedComponent :type Primitive%20Component%20Object%20Reference) (OtherActor :type Actor%20Object%20Reference) (OtherComp :type Primitive%20Component%20Object%20Reference) (OtherBodyIndex :type Integer) (bFromSweep :type Boolean) (SweepResult :type Hit%20Result%20Structure%20%28by%20ref%29))
  (bind _returnvalue (Components|GetOwner))
  (if (not (== OtherActor _returnvalue))
    ;[1 1 1] ifin circle
    (if (Utilities|Name|Equal(Name) (Variables|Default|Getcolourname) (Variables|/Game/ThirdPersonBP/Blueprints/ThirdPersonCharacter.ThirdPersonCharacter_C|GetColourPlayerIsIn (Variables|Default|GetPlayer%20Reference)))
      (Development|PrintString "Player was in circle, no bug" true true "(R=1.000000,G=0.000000,B=0.008232,A=1.000000)")
      (else
        (Game|Damage|ApplyDamage OtherActor 1e+01 0 _returnvalue)))))

(event EventBeginPlay
  (|CallParentFunction)
  (switch int (Math|Random|RandomIntegerinRange 0 3)
    (:0
      (Development|PrintString "skyorbred")
      (Variables|Default|Setcolour "(R=1.000000,G=0.015783,B=0.000000,A=1.000000)")
      (Variables|Default|Setcolourname "red"))
    (:1
      (Development|PrintString "skyorbblue")
      (Variables|Default|Setcolour "(R=0.014323,G=0.000000,B=1.000000,A=1.000000)")
      (Variables|Default|Setcolourname "blue"))
    (:2
      (Development|PrintString "skyorbyellow")
      (Variables|Default|Setcolour "(R=1.000000,G=0.689642,B=0.000000,A=1.000000)")
      (Variables|Default|Setcolourname "yellow"))
    (:3
      (Development|PrintString "skyorbgreen")
      (Variables|Default|Setcolour "(R=0.000000,G=1.000000,B=0.083799,A=1.000000)")
      (Variables|Default|Setcolourname "green")))
  (Effects|Components|ParticleSystem|SetVectorParameter (Variables|Default|GetFX) "color" (Math|Conversions|ToVector(LinearColor) (Variables|Default|Getcolour)))
  (bind _returnvalue (Actor|GetActorOfClass "/Game/ThirdPersonBP/Blueprints/ThirdPersonCharacter.ThirdPersonCharacter_C"))
  (Variables|Default|SetPlayer%20Reference _returnvalue)
  (Variables|/Script/Engine.ProjectileMovementComponent|SetHomingTargetComponent (Variables|Default|GetProjectileMovement) (Variables|/Script/Engine.Actor|GetRootComponent (Game|Player|GetPlayerPawn 0)))
  (Utilities|FlowControl|Delay 7.0)
  (Actor|DestroyActor))

(fn ConstructionScript
  (|CallParentFunction))