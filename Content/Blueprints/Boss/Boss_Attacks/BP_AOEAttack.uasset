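; BP_AOEAttack is a short-lived area-of-effect attack actor for a boss that damages actors it overlaps, excluding its owner.
; After a brief delay on spawn, it enables overlap on its collision component, plays an embedded Actor Sequence, then destroys itself.
; Sequencer event endpoints time the attached whoosh sound and switch collision off, so the sequence controls when the damage window closes.
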(event OnComponentBeginOverlap(Collision)
  (params (OverlappedComponent :type Primitive%20Component%20Object%20Reference) (OtherActor :type Actor%20Object%20Reference) (OtherComp :type Primitive%20Component%20Object%20Reference) (OtherBodyIndex :type Integer) (bFromSweep :type Boolean) (SweepResult :type Hit%20Result%20Structure%20%28by%20ref%29))
  (bind _returnvalue (Components|GetOwner))
  (if (not (== OtherActor _returnvalue))
    (Game|Damage|ApplyDamage OtherActor 1e+01 0 _returnvalue)))

(event EventBeginPlay
  (Utilities|FlowControl|Delay 1.0)
  (Collision|SetCollisionProfileName (Variables|Default|GetCollision) "OverlapAllDynamic" true :!class /Script/Engine.PrimitiveComponent)
  (Sequencer|Player|Play (Variables|/Script/ActorSequence.ActorSequenceComponent|GetSequencePlayer (Variables|Default|GetActorSequence)) :!class /Script/MovieScene.MovieSceneSequencePlayer)
  (Utilities|FlowControl|Delay 2.0)
  (Actor|DestroyActor))

(event Custom|Whoosh%20sound
  (params (Sphere :type Static%20Mesh%20Component%20Object%20Reference))
  (Audio|SpawnSoundAttached "/Game/Audio/SFX/SoundCues/SC_SFX_Boss_RisingIntoAir.SC_SFX_Boss_RisingIntoAir" (Variables|Default|GetCollision) "None" "0, 0, 0" "0, 0, 0" "KeepRelativeOffset" false 3.0 1.0 0.0 0 0))

(event Custom|DisableCollision
  (params (Sphere :type Static%20Mesh%20Component%20Object%20Reference))
  (Collision|SetCollisionProfileName (Variables|Default|GetCollision) "NoCollision" true :!class /Script/Engine.PrimitiveComponent))

(fn ConstructionScript)