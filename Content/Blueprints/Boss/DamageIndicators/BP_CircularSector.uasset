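; BP_CircularSector is a boss attack indicator that shows a circular sector filling up before an explosion.
; On BeginPlay it creates dynamic materials for the Circum and Area components, set to outline and fill modes with a shared sector angle.
; After a delay, a timeline animates the Area fill, then it spawns an explosion particle and destroys its spawner and itself.
; It applies no damage itself.
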(event EventBeginPlay
  (Utilities|FlowControl|Sequence
    (:then_0
      (bind _returnvalue (Rendering|Material|CreateDynamicMaterialInstance (Variables|Default|GetCircum) :!class /Script/Engine.DecalComponent))
      (bind _output_get (Variables|Default|SetCircumRef _returnvalue))
      (Rendering|Material|SetScalarParameterValue _output_get "Cicum1Area0" 1.0 :!class /Script/Engine.MaterialInstanceDynamic))
    (:then_1
      (bind _returnvalue_2 (Rendering|Material|CreateDynamicMaterialInstance (Variables|Default|GetArea) :!class /Script/Engine.DecalComponent))
      (bind _output_get_2 (Variables|Default|SetAreaRef _returnvalue_2))
      (Rendering|Material|SetScalarParameterValue _output_get_2 "Cicum1Area0" 0.0 :!class /Script/Engine.MaterialInstanceDynamic))
    (:then_2
      (Rendering|Material|SetScalarParameterValue (Variables|Default|GetAreaRef) "RadianValue" 0.25 :!class /Script/Engine.MaterialInstanceDynamic))
    (:then_3
      (Utilities|FlowControl|Delay 1.0)
      (bind _areavaluealpha (Timeline|AreaValueTimeline Play)
        (:Update
          (Rendering|Material|SetScalarParameterValue (Variables|Default|GetAreaRef) "AreaValue" _areavaluealpha :!class /Script/Engine.MaterialInstanceDynamic))
        (:Finished
          (Utilities|FlowControl|Delay 0.1)
          (Effects|SpawnEmitteratLocation "/Game/StarterContent/Particles/P_Explosion.P_Explosion" (Transformation|GetActorLocation) "0, 0, 0" "3.000000,3.000000,3.000000")
          (Actor|DestroyActor (Variables|Default|GetSpawnerRef))
          (Actor|DestroyActor))))))

(fn ConstructionScript)