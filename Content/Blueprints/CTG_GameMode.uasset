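; Game mode that relays popup and win/lose events to the HUD's main widget and records save-slot stats for a boss game.
; After a short startup delay it caches the widget and game instance, binds its listener events and re-broadcasts popup execute results.
; Its timer adds time played, using time-of-day differences, then restarts.
; Game end stops the timer, then saves boss kills, unique boss names or deaths.
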(event Custom|EndTimer
  (bind _gameinstance (Variables|Default|GetGameInstance))
  (bind _gameinstance_2 (Variables|Default|GetGameInstance))
  ;[1 1 1] Begin Play
  ;;[1 1 1] End Timer Event
  (Variables|Default|SetElapsedTime (Math|DateTime|Now))
  (Utilities|Struct|SetmembersinBP_Struct_SaveData (Utilities|Array|Get(acopy) (Variables|/Game/Blueprints/SaveData/BP_PlayerSaveData.BP_PlayerSaveData_C|GetSaves (Variables|/Game/Blueprints/SaveData/BP_SaveGameInstance.BP_SaveGameInstance_C|GetSaveGameData _gameinstance_2)) (Variables|/Game/Blueprints/SaveData/BP_SaveGameInstance.BP_SaveGameInstance_C|GetLoadedSaveIndex _gameinstance_2)) (+ (Utilities|Struct|BreakBP_Struct_SaveData (Variables|/Game/Blueprints/SaveData/BP_SaveGameInstance.BP_SaveGameInstance_C|GetLoadedSave (Variables|Default|GetGameInstance))) (Math|Timespan|GetTotalSeconds (- (TimeOfDay|GetTimeOfDay (Variables|Default|GetElapsedTime) :!class /Script/Engine.KismetMathLibrary) (TimeOfDay|GetTimeOfDay (Variables|Default|GetStartTime) :!class /Script/Engine.KismetMathLibrary)))))
  (SaveGame|SaveGametoSlot (Variables|/Game/Blueprints/SaveData/BP_SaveGameInstance.BP_SaveGameInstance_C|GetSaveGameData _gameinstance) (Variables|/Game/Blueprints/SaveData/BP_SaveGameInstance.BP_SaveGameInstance_C|GetSaveGameSlot _gameinstance))
  (CallFunction|StartTimer))

(event Custom|StartTimer
  ;[1 1 1] Begin Play
  ;;[1 1 1] Start Timer Event
  (Variables|Default|SetStartTime (Math|DateTime|Now)))

(event Custom|OpenPopupWidget
  (params (DialogueText :type Array%20of%20Texts) (ExecuteCode :type String) (bPauseGame? :type Boolean))
  ;[1 1 1] Begin Play
  ;;[1 1 1] Open Popup Widget Event
  (Default|CallEventListenerCreatePopupWidget (Variables|Default|GetMainWidgetReference) DialogueText ExecuteCode bPauseGame?))

(event Custom|OpenWinLoseScreen
  (params (WhichScreen? :type En_WinOrLoseScreen%20Enum :default "NewEnumerator0"))
  ;[1 1 1] Begin Play
  ;;[1 1 1] Open Win/Lose Screen Event
  (Default|CallEventListenerCreateWinLoseScreen (Variables|Default|GetMainWidgetReference) WhichScreen?)
  (CallFunction|EndTimer)
  (CallFunction|WinLoseGame WhichScreen?))

(event Custom|Win%20Lose%20Game
  (params (WhichScreen? :type En_WinOrLoseScreen%20Enum :default "NewEnumerator0"))
  (bind _gameinstance (Variables|Default|GetGameInstance))
  (bind _gameinstance_2 (Variables|Default|GetGameInstance))
  (bind _gameinstance_3 (Variables|Default|GetGameInstance))
  (bind _loadedsave (Variables|/Game/Blueprints/SaveData/BP_SaveGameInstance.BP_SaveGameInstance_C|GetLoadedSave _gameinstance))
  (bind (_bosseskilled _uniquebosseskilled) (Utilities|Struct|BreakBP_Struct_SaveData _loadedsave))
  ;[1 1 1] Win/Lose Game
  (switch Utilities|FlowControl|Switch|SwitchonEn_WinOrLoseScreen WhichScreen?
    (:NewEnumerator0
      (bind _returnvalue (Actor|GetActorOfClass "/Game/Blueprints/Boss/Boss_Class.Boss_Class_C"))
      (bind _output_get (Variables|Default|SetTempSaveData _uniquebosseskilled))
      (if (not (Utilities|Array|ContainsItem _output_get (Variables|/Game/Blueprints/Boss/Boss_Class.Boss_Class_C|GetBossName _returnvalue)))
        (Utilities|Array|Add (Variables|Default|GetTempSaveData) (Variables|/Game/Blueprints/Boss/Boss_Class.Boss_Class_C|GetBossName _returnvalue)))
      (Utilities|Struct|SetmembersinBP_Struct_SaveData (Utilities|Array|Get(acopy) (Variables|/Game/Blueprints/SaveData/BP_PlayerSaveData.BP_PlayerSaveData_C|GetSaves (Variables|/Game/Blueprints/SaveData/BP_SaveGameInstance.BP_SaveGameInstance_C|GetSaveGameData _gameinstance)) (Variables|/Game/Blueprints/SaveData/BP_SaveGameInstance.BP_SaveGameInstance_C|GetLoadedSaveIndex _gameinstance)) (+ _bosseskilled 1) (Variables|Default|GetTempSaveData)))
    (:NewEnumerator1
      (Utilities|Struct|SetmembersinBP_Struct_SaveData (Utilities|Array|Get(acopy) (Variables|/Game/Blueprints/SaveData/BP_PlayerSaveData.BP_PlayerSaveData_C|GetSaves (Variables|/Game/Blueprints/SaveData/BP_SaveGameInstance.BP_SaveGameInstance_C|GetSaveGameData _gameinstance_2)) (Variables|/Game/Blueprints/SaveData/BP_SaveGameInstance.BP_SaveGameInstance_C|GetLoadedSaveIndex _gameinstance_2)) (+ (Utilities|Struct|BreakBP_Struct_SaveData (Variables|/Game/Blueprints/SaveData/BP_SaveGameInstance.BP_SaveGameInstance_C|GetLoadedSave _gameinstance_2)) 1))))
  (SaveGame|SaveGametoSlot (Variables|/Game/Blueprints/SaveData/BP_SaveGameInstance.BP_SaveGameInstance_C|GetSaveGameData _gameinstance_3) (Variables|/Game/Blueprints/SaveData/BP_SaveGameInstance.BP_SaveGameInstance_C|GetSaveGameSlot _gameinstance_3)))

(event Custom|PopupWidgetExecute
  (params (ExecuteCode :type String) (ExecuteIndex :type Integer))
  ;[1 1 1] Begin Play
  ;;[1 1 1] Trigger Dialogue Execute
  (Default|CallEventDispatcherPopupWidgetExecute ExecuteCode ExecuteIndex))

(event EventBeginPlay
  ;[1 1 1] Begin Play
  (Variables|Default|SetStartTime (Math|DateTime|Now))
  (Utilities|FlowControl|Delay 0.5)
  (Utilities|FlowControl|Sequence
    (:then_0
      ;;[1 1 1] Casts
      (bind _ashud_main (Utilities|Casting|CastToHUD_Main (HUD|GetHUD (Game|GetPlayerController 0))))
      (Variables|Default|SetMainWidgetReference (Variables|/Game/Widgets/HUD_Main.HUD_Main_C|GetMainWidgetReference _ashud_main))
      (bind _asbp_save_game_instance (Utilities|Casting|CastToBP_SaveGameInstance (Game|GetGameInstance)))
      (Variables|Default|SetGameInstance _asbp_save_game_instance))
    (:then_1
      (EventDispatchers|BindEventtoEventListenerEndTimer (delegate Custom|EndTimer))
      (EventDispatchers|BindEventtoEventListenerStartTimer (delegate Custom|StartTimer))
      (EventDispatchers|BindEventtoEventListenerOpenPopupWidget (delegate Custom|OpenPopupWidget))
      (EventDispatchers|BindEventtoEventListenerOpenWinLoseScreen (delegate Custom|OpenWinLoseScreen))
      (EventDispatchers|BindEventtoEventDispatcherPopupWidgetExecute (Variables|Default|GetMainWidgetReference) (delegate Custom|PopupWidgetExecute)))))

(fn ConstructionScript)