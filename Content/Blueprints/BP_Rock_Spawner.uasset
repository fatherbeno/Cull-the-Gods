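; Rock spawner actor that scatters instanced meshes in a random cubic volume and spins them as a group.
; The construction script creates one HISM component per SMBlocks mesh, then adds instances with random location, rotation and non-uniform scale.
; The seeded stream drives only location and scale; mesh choice, which never selects the last entry, and rotation are unseeded.
; Tick applies the Rotation increment to the root after a delta-time Delay.
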(event EventBeginPlay)

(event Collision|EventActorBeginOverlap
  (params (OtherActor :type Actor%20Object%20Reference)))

(event EventTick
  (params (DeltaSeconds :type Float%20%28single-precision%29))
  (bind _defaultsceneroot (Variables|Default|GetDefaultSceneRoot))
  (Utilities|FlowControl|Delay DeltaSeconds)
  (Transformation|SetWorldRotation _defaultsceneroot (Math|Rotator|CombineRotators (Transformation|GetWorldRotation _defaultsceneroot) (Variables|Default|GetRotation)) false false))

(fn ConstructionScript
  (bind _random_stream (Variables|Default|GetRandom%20Stream))
  (bind _spawn_min (Variables|Default|GetSpawn%20Min))
  (bind _hism_blocks (Variables|Default|GetHISM%20Blocks))
  (bind _scale_max (Variables|Default|GetScale%20Max))
  (bind _scale_min (Variables|Default|GetScale%20Min))
  (bind _spawn_max (Variables|Default|GetSpawn%20Max))
  (bind _returnvalue (Math|Random|RandomFloatinRangefromStream _scale_min _scale_max _random_stream))
  (Math|Random|SetRandomStreamSeed (Variables|Default|GetRandom%20Stream) (Variables|Default|GetSeed))
  (for _array_element (Variables|Default|GetSM%20Blocks)
    (bind _returnvalue_2 (AddComponent|AddHierarchicalInstancedStaticMeshComponent false))
    (Components|StaticMesh|SetStaticMesh _returnvalue_2 _array_element)
    (Utilities|Array|Add _hism_blocks _returnvalue_2))
  (for _index (range 0 (Variables|Default|GetNumber%20of%20Blocks))
    (Components|InstancedStaticMesh|AddInstance (Utilities|Array|Get(acopy) _hism_blocks (Math|Random|RandomInteger (- (Utilities|Array|Length _hism_blocks) 1))) (Math|Transform|MakeTransform (Math|Vector|MakeVector (Math|Random|RandomFloatinRangefromStream _spawn_min _spawn_max _random_stream) (Math|Random|RandomFloatinRangefromStream _spawn_min _spawn_max _random_stream) (Math|Random|RandomFloatinRangefromStream _spawn_min _spawn_max _random_stream)) (Math|Random|RandomRotator true) (Math|Vector|MakeVector _returnvalue _returnvalue _returnvalue)))))